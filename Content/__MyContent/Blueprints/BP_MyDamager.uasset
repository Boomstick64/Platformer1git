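; BP_MyDamager is a volume that damages a player-tagged ThirdPersonCharacter through its ChangeHealth function.
; Entering CollisionVolume deals instant damage capped at a maximum and restarts the accumulated total.
; While the player stays inside, Tick applies frame-rate-scaled damage until that total reaches the maximum, which the final tick can slightly overshoot.
; Leaving stops the damage, and each re-entry starts a fresh cycle.
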(event `self.ReceiveTick`
  (params (DeltaSeconds :type "Float (single-precision)"))
  (if (`self.Inside Volume`)
    (`self.Continue Damage`)))

(event `self.Collision volume.OnComponentBeginOverlap`
  (params (OverlappedComponent :type "PrimitiveComponent Object Reference") (OtherActor :type "Actor Object Reference") (OtherComp :type "PrimitiveComponent Object Reference") (OtherBodyIndex :type Integer) (bFromSweep :type Boolean) (SweepResult :type "HitResult Structure (by ref)"))
  (if (`self.ActorHasTag` OtherActor "Tag_Player")
    (bind _asthird_person_character (cast `/Game/ThirdPersonBP/Blueprints/ThirdPersonCharacter` OtherActor))
    (set `self.Inside Volume` true)
    (set `self.Player` _asthird_person_character)
    (`self.Start Damage`)))

(event `self.Collision volume.OnComponentEndOverlap`
  (params (OverlappedComponent :type "PrimitiveComponent Object Reference") (OtherActor :type "Actor Object Reference") (OtherComp :type "PrimitiveComponent Object Reference") (OtherBodyIndex :type Integer))
  (if (`self.ActorHasTag` OtherActor "Tag_Player")
    (cast `/Game/ThirdPersonBP/Blueprints/ThirdPersonCharacter` OtherActor)
    (set `self.Inside Volume` false)))

(fn `Continue Damage`
  (bind _returnvalue (* (`self.Damage Rate`) (`GameplayStatics.GetWorldDeltaSeconds`)))
  (if (< (`self.Accumalitive Damage`) (`self.Max Damage`))
    (set `self.Accumalitive Damage` (+ _returnvalue (`self.Accumalitive Damage`))) ; Increase accum damage by damage rate
    (`/Game/ThirdPersonBP/Blueprints/ThirdPersonCharacter.Change Health` (`self.Player`) (* _returnvalue -1.0))))

(fn `Start Damage`
  (bind _output_get (set `self.Accumalitive Damage` (`self.Instant Damage`)))
  (if (> _output_get (`self.Max Damage`))
    (set `self.Accumalitive Damage` (`self.Max Damage`)))
  (`/Game/ThirdPersonBP/Blueprints/ThirdPersonCharacter.Change Health` (`self.Player`) (* (`self.Accumalitive Damage`) -1.0)))

(fn `UserConstructionScript`)