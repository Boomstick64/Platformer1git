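; BP_EnemySpawn is a one-shot trigger that spawns a batch of enemies inside an area.
; The first overlap on its Visibility component calls SpawnEnemy SpawnAmount times.
; Each call traces down against WorldStatic from high above a random point in Spawnbounds, with debug drawing enabled.
; It spawns BP_Enemy1 slightly above the hit location without checking for a hit, then gives it a default controller.
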(event `self.Visibility.OnComponentBeginOverlap`
  (params (OverlappedComponent :type "PrimitiveComponent Object Reference") (OtherActor :type "Actor Object Reference") (OtherComp :type "PrimitiveComponent Object Reference") (OtherBodyIndex :type Integer) (bFromSweep :type Boolean) (SweepResult :type "HitResult Structure (by ref)"))
  (bind _counter (`/Engine/EditorBlueprintResources/StandardMacros.Do N` 1)
    (:`Exit`
      (switch `int` _counter
        (:`1`
          (for _ (range 1 (+ (`self.spawn amount`) 1))
            (`self.Spawn Enemy`)))))))

(fn `Spawn Enemy`
  (bind (_origin _boxextent) (`KismetSystemLibrary.GetComponentBounds` (`self.spawnbounds`)))
  (bind _returnvalue (`KismetMathLibrary.MakeVector` (.x (`KismetMathLibrary.RandomPointInBoundingBox` _origin _boxextent)) (.y (`KismetMathLibrary.RandomPointInBoundingBox` _origin _boxextent)) (+ (.z (`KismetMathLibrary.RandomPointInBoundingBox` _origin _boxextent)) 10000.0)))
  (bind _outhit (`KismetSystemLibrary.LineTraceSingleForObjects` :`Start` _returnvalue :`End` (+ _returnvalue (* (* (`self.GetActorUpVector`) -1) 15000.0)) :`ObjectTypes` (`|MakeArray` "ObjectTypeQuery1" :!type "EObjectTypeQuery Enum") :`DrawDebugType` "ForDuration"))
  (bind _returnvalue_2 (`|SpawnActorFromClass` "/Game/ThirdPersonBP/Blueprints/BP_Enemy1.BP_Enemy1_C" (`KismetMathLibrary.MakeTransform` (`KismetMathLibrary.MakeVector` (.x (`.Location` (`GameplayStatics.BreakHitResult` _outhit))) (.y (`.Location` (`GameplayStatics.BreakHitResult` _outhit))) (+ (.z (`.Location` (`GameplayStatics.BreakHitResult` _outhit))) 100.0))) "AdjustIfPossibleButAlwaysSpawn" "OverrideRootScale" null null))
  (`Pawn.SpawnDefaultController` _returnvalue_2))

(fn `UserConstructionScript`)