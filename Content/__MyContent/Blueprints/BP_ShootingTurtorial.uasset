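; Trigger-box actor that shows the shooting tutorial when the third-person character walks into it.
; Box overlaps pass through a DoN counter, and only the count of one runs the tutorial.
; It sets the game manager's state, hides other UI, enables the HUD and shows the shooting tutorial widget, then hides that widget after a timed delay.
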(event `self.Box.OnComponentBeginOverlap`
  (params (OverlappedComponent :type "PrimitiveComponent Object Reference") (OtherActor :type "Actor Object Reference") (OtherComp :type "PrimitiveComponent Object Reference") (OtherBodyIndex :type Integer) (bFromSweep :type Boolean) (SweepResult :type "HitResult Structure (by ref)"))
  (cast `/Game/ThirdPersonBP/Blueprints/ThirdPersonCharacter` OtherActor)
  (bind _counter (`/Engine/EditorBlueprintResources/StandardMacros.Do N` 2)
    (:`Exit`
      (switch `int` _counter
        (:`1`
          (bind _my_game_manager (`/Game/__MyContent/Blueprints/BP_MyFunctionLibrary.Get My Game Manager`))
          (`/Game/__MyContent/Blueprints/BP_MyGameManager.Set State` _my_game_manager "NewEnumerator0")
          (`/Game/__MyContent/Blueprints/BP_MyFunctionLibrary.Hide UI`)
          (`/Game/__MyContent/Blueprints/BP_MyGameManager.Show HUD` _my_game_manager true)
          (bind _widget_shooting_turtorial (`/Game/__MyContent/Blueprints/BP_MyGameManager.Widget Shooting Turtorial` _my_game_manager))
          (`Widget.SetVisibility` _widget_shooting_turtorial "Visible")
          (`KismetSystemLibrary.Delay` 10.0)
          (`Widget.SetVisibility` _widget_shooting_turtorial "Hidden"))))))

(fn `UserConstructionScript`)